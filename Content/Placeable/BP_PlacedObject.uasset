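; Placeable product actor that can be moved, rotated and scaled on a detected or referenced plane actor through screen-space input.
; Construction applies the referenced product asset's mesh and sizes its base plate.
; Positioning deprojects a screen point and moves the object only when the trace hits BPPlane.
; Rotation yaws against horizontal drag while accumulating travel distance; scaling steps by the sign of input change within clamped limits.
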(fn `AssignProductAsset`
  (bind _bp_productassetref (`self.BP_ProductAssetRef`))
  (bind _platescale (`/Game/Placeable/BP_ProductAssetRef.PlateScale` _bp_productassetref))
  (`StaticMeshComponent.SetStaticMesh` (`self.SM_Object`) (`/Game/Placeable/BP_ProductAssetRef.StaticMesh` _bp_productassetref))
  (`SceneComponent.SetWorldScale3D` (`self.SM_Plane`) (`KismetMathLibrary.MakeVector` _platescale _platescale 0.0)))

(fn `SetPlaceablePosition`
  (params (Location :type "Vector2D Structure"))
  (bind (_worldposition _worlddirection) (`GameplayStatics.DeprojectScreenToWorld` (`GameplayStatics.GetPlayerController` 0) Location))
  (bind (_outhit _returnvalue) (`KismetSystemLibrary.LineTraceSingleForObjects` _worldposition (+ _worldposition (* _worlddirection 1000.0)) (`|MakeArray` "ObjectTypeQuery1" "ObjectTypeQuery2" "ObjectTypeQuery3" "ObjectTypeQuery4" "ObjectTypeQuery5" "ObjectTypeQuery6" :!type "EObjectTypeQuery Enum")))
  (if _returnvalue
    (bind (_bblockinghit _binitialoverlap _time _distance _location _impactpoint _normal _impactnormal _physmat _hitactor) (`GameplayStatics.BreakHitResult` _outhit))
    (if (== _hitactor (`self.BP_Plane`))
      (`SceneComponent.K2_SetWorldLocation` (`self.Placeable`) _location false false))))

(fn `SetPlaceableRotation`
  (params (Direction :type "Vector2D Structure") (Location :type "Vector2D Structure"))
  (set `self.DistanceTravelled` (+ (`KismetMathLibrary.Distance2D` (`local.Location`) (`self.PreviousLocation`)) (`self.DistanceTravelled`)))
  (set `self.PreviousLocation` (`local.Location`))
  (`SceneComponent.K2_AddRelativeRotation` (`self.Placeable`) (`KismetMathLibrary.MakeRotator` 0.0 0.0 (* (`KismetMathLibrary.BreakVector2D` (`local.Direction`)) -1.0)) false false))

(fn `SetPlaceableScale`
  (params (NewScaleMapping :type "Float (double-precision)"))
  (bind _output_get (set `self.PreviousPlaceableScale` (`KismetMathLibrary.FClamp` (+ (* (`KismetMathLibrary.SignOfFloat` (- (`local.NewScaleMapping`) (`self.PreviousScaleMapping`))) 0.01) (`self.PreviousPlaceableScale`)) 0.5 1.5)))
  (`SceneComponent.SetWorldScale3D` (`self.Placeable`) (`KismetMathLibrary.MakeVector` _output_get _output_get _output_get))
  (set `self.PreviousScaleMapping` (`local.NewScaleMapping`)))

(fn `UserConstructionScript`
  (`self.AssignProductAsset`))