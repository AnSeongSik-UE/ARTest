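; BP_Plane is a placeable flat plane with functions for other code to show, hide, scale and re-material it.
; BeginPlay creates a dynamic instance of M_Plane_Plain and stores it in DMPlane, which is only applied to the Plane component when SwitchToMaterial runs.
; SetScale takes X and Y from its input and forces the relative Z scale to zero.
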(event `self.ReceiveBeginPlay`
  (bind _returnvalue (`KismetMaterialLibrary.CreateDynamicMaterialInstance` "/Game/Placeable/Materials/M_Plane_Plain.M_Plane_Plain"))
  (set `self.DM_Plane` _returnvalue))

(fn `Hide`
  (`SceneComponent.SetVisibility` (`self.Plane`) false false))

(fn `SetScale`
  (params (Scale :type "Vector Structure"))
  (`SceneComponent.SetRelativeScale3D` (`self.Plane`) (`KismetMathLibrary.MakeVector` (.x Scale) (.y Scale))))

(fn `Show`
  (`SceneComponent.SetVisibility` (`self.Plane`) true false))

(fn `SwitchToMaterial`
  (`PrimitiveComponent.SetMaterial` (`self.Plane`) 0 (`self.DM_Plane`)))

(fn `UserConstructionScript`)