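; AR player pawn that creates the main menu and lets the player place and manipulate one object on a detected plane.
; After scanning, a screen-center AR trace refreshes a spawned candidate plane every second.
; Touch traces select that plane, then spawn the object on it.
; Timer-debounced gestures drive the object: one finger moves it, while two fingers rotate or scale it by horizontal or vertical drag direction.
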(event `self.ReceiveBeginPlay`
  ; HUD 생성
  (bind _returnvalue (`|CreateWidget` "/Game/UI/BP_MainMenu.BP_MainMenu_C" (`GameplayStatics.GetPlayerController` 0)))
  (bind _output_get (set `self.MainMenu` _returnvalue))
  (`UserWidget.AddToViewport` _output_get 0))

(event `self.ReceiveTick`
  (params (DeltaSeconds :type "Float (single-precision)"))
  (bind _returnvalue (`self.GetInputAxisValue`))
  (set `self.DT` DeltaSeconds)
  (`|ExecutionSequence`
    (:`then_0`
      (`self.ResetRecognisedGesture`)
      (`self.OneFingerGestureRecognition`)
      (`self.TwoFingerGestureRecognition`)
      (`self.GestureRecognised`
        (:`then`
          (switch `/Game/GameFramework/E_GestureType` (`self.CurrentTransformation`)
            (:`NewEnumerator0`
              (`/Game/Placeable/BP_PlacedObject.SetPlaceablePosition` (`self.PlacedObject`) (`self.GetTouchLocation`)))
            (:`NewEnumerator1`
              (`/Game/Placeable/BP_PlacedObject.SetPlaceableRotation` (`self.PlacedObject`) (`self.GetFingerDirection`) (`self.GetTouchLocation`)))
            (:`NewEnumerator2`
              (`/Game/Placeable/BP_PlacedObject.SetPlaceableScale` (`self.PlacedObject`) _returnvalue)
              (`KismetSystemLibrary.PrintString` (`KismetStringLibrary.Concat_StrStr` "TFM:" (`KismetStringLibrary.Conv_DoubleToString` _returnvalue))))))
        (:`else`)))
    (:`then_1`
      (if (not (`self.ScanningIsDone`))
        (`self.DepthTexture`
          (:`then`)
          (:`else`
            (bind _returnvalue_2 (`ARBlueprintLibrary.GetARTexture` "SceneDepthMap"))
            (set `self.DepthTexture` _returnvalue_2)))))
    (:`then_2`
      ; 바닥 만들기
      (if (and (`self.ScanningIsDone`) (not (`self.PlaneIsSelected`)))
        (bind _output_get (set `self.ShowPlaneTimer` (+ (`self.DT`) (`self.ShowPlaneTimer`))))
        (if (> _output_get 1.0)
          (set `self.ShowPlaneTimer` 0.0)
          (`self.UpdatePlaneCandidate`))))))

(event `InputTouch`
  (params (Location :type "Vector Structure") (FingerIndex :type "ETouchIndex Enum"))
  (bind _selectedplane (`self.SelectedPlane`))
  (:`Pressed`
    (switch `ETouchIndex` FingerIndex
      (:`Touch1`
        (`self.PlaneIsSelected`
          (:`then`
            (if (not (`self.ObjectIsPlaced`))
              (bind (_outhit _returnvalue) (`self.WorldHitTest` (`self.GetTouchLocation`)))
              (if _returnvalue
                (bind (_bblockinghit _binitialoverlap _time _distance _location _impactpoint _normal _impactnormal _physmat _hitactor) (`GameplayStatics.BreakHitResult` _outhit))
                (if (== (`self.SelectedPlane`) _hitactor)
                  (bind _returnvalue_2 (`|SpawnActorFromClass` "/Game/Placeable/BP_PlacedObject.BP_PlacedObject_C" (`KismetMathLibrary.Conv_VectorToTransform` _location) "Undefined" "MultiplyWithRoot" null null))
                  (bind _output_get (set `self.PlacedObject` _returnvalue_2))
                  (set `/Game/Placeable/BP_PlacedObject.BP_Plane` _selectedplane _output_get)
                  (set `self.ObjectIsPlaced` true)
                  (`/Game/Placeable/BP_Plane.Hide` _selectedplane)
                  (`self.ARObjectSpawned`)))
              (else
                (`KismetSystemLibrary.PrintString` "ObjectNotPlaced"))))
          (:`else`
            (`KismetSystemLibrary.PrintString` "StartPlaneSelect")
            ; 라인트레이스 진행, 리절트 변환
            (bind (_outhit_2 _returnvalue_3) (`self.WorldHitTest` (`self.GetTouchLocation`)))
            (if _returnvalue_3
              (bind _asbp_plane (cast `/Game/Placeable/BP_Plane` (`.HitActor` (`GameplayStatics.BreakHitResult` _outhit_2)))
                (:`then`
                  (`/Engine/EditorBlueprintResources/StandardMacros.IsValid` (`/Game/Placeable/BP_Plane.Plane` _asbp_plane)
                    (:`Is Valid`
                      (bind _output_get_2 (set `self.SelectedPlane` _asbp_plane))
                      (`self.BPPlaneSelected` _output_get_2)
                      (set `self.PlaneIsSelected` true)
                      (`KismetSystemLibrary.PrintString` "PlaneSelected"))
                    (:`Is Not Valid`
                      (`KismetSystemLibrary.PrintString` "PlaneNotValid"))))
                (:`CastFailed`
                  (`KismetSystemLibrary.PrintString` "PlaneCastFalse")))
              (else
                (`KismetSystemLibrary.PrintString` "PlaneSelectFalse")))))))))

(event `InputAction|OneFingerAction`
  (params (Key :type "Key Structure"))
  (:`Pressed`
    (bind _outhit (`self.WorldHitTest` (`self.GetTouchLocation`)))
    (cast `/Game/Placeable/BP_PlacedObject` (`.HitActor` (`GameplayStatics.BreakHitResult` _outhit)))
    (set `self.OneFingerPressed` true)
    (set `self.OneFingerValidationTimer` 0.0))
  (:`Released`
    (set `self.OneFingerPressed` false)))

(event `InputAction|TwoFingerAction`
  (params (Key :type "Key Structure"))
  (bind _location (`self.GetTouchLocation`))
  (:`Pressed`
    (set `self.TwoFingerPressed` true)
    (set `self.TwoFingerValidationTimer` 0.0)
    (set `self.PreviousFingerPosition` _location)
    (set `self.StartingFingerPosition` _location)
    (set `self.PreviousFingerDistance` (`self.GetFingerDistance`)))
  (:`Released`
    (set `self.TwoFingerPressed` false)))

(fn `AnyTouchReceived`
  (returns (ReturnValue :type Boolean))
  (bind _returnvalue (`GameplayStatics.GetPlayerController` 0))
  (return (or (`.bIsCurrentlyPressed` (`PlayerController.GetInputTouchState` _returnvalue "Touch1")) (`.bIsCurrentlyPressed` (`PlayerController.GetInputTouchState` _returnvalue "Touch2")))))

(fn `CreatePlaneCandidate`
  (params (ARPlaneGeo :type "ARPlaneGeometry Object Reference") (ARTrackedGeo :type "ARTrackedGeometry Object Reference"))
  (returns (Plane :type "/Game/Placeable/BP_Plane Object Reference"))
  (bind _returnvalue (`|SpawnActorFromClass` "/Game/Placeable/BP_Plane.BP_Plane_C" (`ARTrackedGeometry.GetLocalToWorldTransform` ARPlaneGeo) "Undefined" "MultiplyWithRoot" null null))
  (`SceneComponent.SetRelativeScale3D` (`/Game/Placeable/BP_Plane.Plane` _returnvalue) (`KismetMathLibrary.MakeVector` (.x (/ (`ARPlaneGeometry.GetExtent` ARPlaneGeo) 50.0)) (.y (/ (`ARPlaneGeometry.GetExtent` ARPlaneGeo) 50.0))))
  (return _returnvalue))

(fn `GetFingerDirection`
  (returns (NormalizedDirection :type "Vector2D Structure"))
  (bind (_locationx _locationy) (`PlayerController.GetInputTouchState` (`GameplayStatics.GetPlayerController` 0) "Touch1"))
  (return (`KismetMathLibrary.Normal2D` (- (`KismetMathLibrary.MakeVector2D` _locationx _locationy) (`self.PreviousFingerPosition`)))))

(fn `GetFingerDistance`
  (returns (FingerDistance :type "Float (double-precision)"))
  (bind _returnvalue (`GameplayStatics.GetPlayerController` 0))
  (bind (_locationx _locationy) (`PlayerController.GetInputTouchState` _returnvalue "Touch2"))
  (bind (_locationx_2 _locationy_2) (`PlayerController.GetInputTouchState` _returnvalue "Touch1"))
  (return (`KismetMathLibrary.Distance2D` (`KismetMathLibrary.MakeVector2D` _locationx_2 _locationy_2) (`KismetMathLibrary.MakeVector2D` _locationx _locationy))))

(fn `GetScreenCenterPosition`
  (returns (CenterPosition :type "Vector2D Structure"))
  (bind (_sizex _sizey) (`PlayerController.GetViewportSize` (`GameplayStatics.GetPlayerController` 0)))
  (return (* (`KismetMathLibrary.MakeVector2D` (`KismetMathLibrary.Conv_IntToDouble` _sizex) (`KismetMathLibrary.Conv_IntToDouble` _sizey)) 0.5)))

(fn `GetTouchLocation`
  (returns (Location :type "Vector2D Structure"))
  (bind (_locationx _locationy) (`PlayerController.GetInputTouchState` (`GameplayStatics.GetPlayerController` 0) "Touch1"))
  (return (`KismetMathLibrary.MakeVector2D` _locationx _locationy)))

(fn `OneFingerGestureRecognition`
  (if (and (`self.ObjectIsPlaced`) (`self.OneFingerPressed`) (not (`self.GestureRecognised`)) (not (`self.TwoFingerPressed`)))
    (bind _output_get (set `self.OneFingerValidationTimer` (+ (`self.DT`) (`self.OneFingerValidationTimer`))))
    (if (> _output_get 0.2)
      (set `self.GestureRecognised` true)
      (set `self.CurrentTransformation` "NewEnumerator0"))
    (else
      (set `self.OneFingerValidationTimer` 0.0))))

(fn `ResetPlacement`
  ; Flag Off
  (set `self.PlaneIsSelected` false)
  (set `self.ObjectIsPlaced` false)
  (`|ExecutionSequence`
    (:`then_0`
      (bind _placedobject (`self.PlacedObject`)
        (:`then`
          (`self.K2_DestroyActor` _placedobject))
        (:`else`)))
    (:`then_1`
      (bind _selectedplane (`self.SelectedPlane`)
        (:`then`
          (`self.K2_DestroyActor` _selectedplane))
        (:`else`)))))

(fn `ResetRecognisedGesture`
  ; 터치 불안정 인식 0.1초 보정
  (`self.GestureRecognised`
    (:`then`
      (if (not (`self.AnyTouchReceived`))
        (bind _output_get (set `self.GestureResetTimer` (+ (`self.DT`) (`self.GestureResetTimer`))))
        (if (> _output_get 0.1)
          (set `self.GestureRecognised` false)
          (set `self.GestureResetTimer` 0.0))
        (else
          (set `self.GestureResetTimer` 0.0))))
    (:`else`)))

(fn `TwoFingerGestureRecognition`
  (if (and (`self.ObjectIsPlaced`) (`self.TwoFingerPressed`) (not (`self.GestureRecognised`)))
    (bind _output_get (set `self.TwoFingerValidationTimer` (+ (`self.DT`) (`self.TwoFingerValidationTimer`))))
    (if (> _output_get 0.2)
      (if (`KismetMathLibrary.NearlyEqual_FloatFloat` (`KismetMathLibrary.Abs` (- (`self.PreviousFingerDistance`) (`self.GetFingerDistance`))) 0.0 0.001)
        (set `self.TwoFingerValidationTimer` 0.0)
        (else
          (set `self.GestureRecognised` true)
          (if (< (`KismetMathLibrary.Abs` (`.Y` (`KismetMathLibrary.BreakVector2D` (`self.GetFingerDirection`)))) 0.5)
            ; 가로이동이 크면 회전
            (set `self.CurrentTransformation` "NewEnumerator1")
            (else
              ; 세로이동이 크면 스케일
              (set `self.CurrentTransformation` "NewEnumerator2"))))))
    (else
      (set `self.TwoFingerValidationTimer` 0.0))))

(fn `UpdatePlaneCandidate`
  ; AR 레이트레이싱
  (bind _returnvalue (`ARBlueprintLibrary.LineTraceTrackedObjects` (`self.GetScreenCenterPosition`) false false))
  (`/Engine/EditorBlueprintResources/StandardMacros.CompareInt` (`KismetArrayLibrary.Array_Length` _returnvalue)
    (:`>`
      (bind _returnvalue_2 (`ARTraceResultLibrary.GetTrackedGeometry` (`|GetArrayItem` _returnvalue)))
      (bind _asarplane_geometry (cast `ARPlaneGeometry` _returnvalue_2)
        (:`then`
          ; 일반레이트레이싱 가능한 바닥면 생성
          (bind _plane (`self.CreatePlaneCandidate` _asarplane_geometry _returnvalue_2))
          (`/Engine/EditorBlueprintResources/StandardMacros.IsValid` _plane
            (:`Is Valid`
              (`|ExecutionSequence`
                (:`then_0`
                  (bind _bpplanecandidate (`self.BPPlaneCandidate`)
                    (:`then`
                      (`self.K2_DestroyActor` _bpplanecandidate))
                    (:`else`)))
                (:`then_1`
                  (set `self.BPPlaneCandidate` _plane)
                  (`KismetSystemLibrary.PrintString` "UpdateCandidateCompleted"))))
            (:`Is Not Valid`
              (`KismetSystemLibrary.PrintString` "CreatedPlaneNotValid"))))
        (:`CastFailed`
          (`KismetSystemLibrary.PrintString` "GeoCastFailed"))))
    (:`==`
      (`KismetSystemLibrary.PrintString` "NotEnoughCandidateAtUpdate" :!label _label))
    (:`<`
      (goto _label))))

(fn `UserConstructionScript`)

(fn `WorldHitTest`
  (params (Location :type "Vector2D Structure"))
  (returns (OutHit :type "HitResult Structure") (ReturnValue :type Boolean))
  (bind (_worldposition _worlddirection) (`GameplayStatics.DeprojectScreenToWorld` (`GameplayStatics.GetPlayerController` 0) Location))
  (bind (_outhit _returnvalue) (`KismetSystemLibrary.LineTraceSingleForObjects` _worldposition (+ _worldposition (* _worlddirection 1000.0)) (`|MakeArray` "ObjectTypeQuery1" "ObjectTypeQuery2" "ObjectTypeQuery3" "ObjectTypeQuery4" "ObjectTypeQuery5" "ObjectTypeQuery6" :!type "EObjectTypeQuery Enum")))
  (return _outhit _returnvalue))